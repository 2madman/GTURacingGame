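; BP_Checkpoint is a checkpoint actor that reports overlaps to the level's finish line.
; On any actor overlap, it looks up the first FinishLine actor and increments its TotalCollision, with no actor filter or repeat guard.
; It also stores the overlapping actor's location and the checkpoint's own yaw there as the last checkpoint position and rotation.
; An unconnected CanFinish array counting branch never runs.
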(event `self.ReceiveActorBeginOverlap`
  (params (OtherActor :type "Actor Object Reference"))
  (bind (_returnvalue_roll _returnvalue_pitch _returnvalue_yaw) (`KismetMathLibrary.BreakRotator` (`self.K2_GetActorRotation`)))
  (bind _outactors (`GameplayStatics.GetAllActorsOfClass` "/Game/Blueprints/FinishLine.FinishLine_C"))
  (set `self.NewVar_0` (`|GetArrayItem` _outactors))
  (`/Engine/EditorBlueprintResources/StandardMacros.IncrementInt` (`/Game/Blueprints/FinishLine.TotalCollision` (`self.NewVar_0`))
    (:`  `
      (set `/Game/Blueprints/FinishLine.lastCheckpoint` (`self.K2_GetActorLocation` OtherActor) (`self.NewVar_0`))
      (set `/Game/Blueprints/FinishLine.lastRotation` _returnvalue_yaw (`self.NewVar_0`)))))

(fn `UserConstructionScript`)