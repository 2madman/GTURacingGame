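; Finish line actor for a two-lap car race that counts laps and ends the game in a win.
; Its trigger, gated by a resettable DoOnce, advances the car's lap UI once TotalCollision reaches a half-race threshold.
; Actor overlap at the full threshold shows the win widget, pauses and switches to UI-only input.
; Live logic here only reads TotalCollision; the checkpoint-based counting nodes are disconnected.
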(event `self.ReceiveActorBeginOverlap`
  (params (OtherActor :type "Actor Object Reference"))
  (bind _returnvalue (`GameplayStatics.GetPlayerController` 0))
  (if (>= (`self.TotalCollision`) 12)
    (set `self.GameWon` true)
    (cast `/Game/VehicleTemplate/Blueprints/SportsCar/SportsCar_Pawn` OtherActor)
    (bind _returnvalue_2 (`|CreateWidget` "/Game/Blueprints/WB_GameWin.WB_GameWin_C"))
    (`UserWidget.AddToViewport` _returnvalue_2 0)
    (set `PlayerController.bShowMouseCursor` true _returnvalue)
    (`GameplayStatics.SetGamePaused` true)
    (`WidgetBlueprintLibrary.SetInputMode_UIOnlyEx` _returnvalue _returnvalue_2)))

(event `self.ReceiveBeginPlay`
  (set `self.lastCheckpoint` (-3490.0 -9330.0 55.93453)))

(event `self.Trigger.OnComponentBeginOverlap`
  (params (OverlappedComponent :type "PrimitiveComponent Object Reference") (OtherActor :type "Actor Object Reference") (OtherComp :type "PrimitiveComponent Object Reference") (OtherBodyIndex :type Integer) (bFromSweep :type Boolean) (SweepResult :type "HitResult Structure (by ref)"))
  ;[1 1 1] Lap counter
  (bind _assports_car_pawn (cast `/Game/VehicleTemplate/Blueprints/SportsCar/SportsCar_Pawn` OtherActor))
  (`/Engine/EditorBlueprintResources/StandardMacros.DoOnce` false :!label _label
    (:`Completed`
      (if (>= (`self.TotalCollision`) 6)
        (if (!= (`self.laps`) 2)
          (`/Engine/EditorBlueprintResources/StandardMacros.IncrementInt` (`self.laps`)
            (:`  `
              (`TextBlock.SetText` (`/Game/Blueprints/WB_LapCounter.Lap_Text` (`/Game/VehicleTemplate/Blueprints/SportsCar/SportsCar_Pawn.lapCounterUI` _assports_car_pawn)) (`|FormatText` "Lap {LapNumber}/2" (`self.laps`)))
              (`KismetSystemLibrary.Delay` 0.7)
              (goto _label :!via `Reset`))))
        (else
          (goto _label :!via `Reset`))))))

(fn `UserConstructionScript`)