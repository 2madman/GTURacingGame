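; BP_Platform is an actor that shakes the camera on overlap and keeps an elapsed minutes-and-seconds timer.
; BeginPlay caches the first FinishLine actor, and overlap plays CS_Deneme at the platform with a debug print.
; Tick uses a Delay as a one-second throttle to count time up.
; A disconnected older countdown, which checks GameWon and shows WB_GameLose at zero, never runs.
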(event `self.ReceiveBeginPlay`
  (bind _outactors (`GameplayStatics.GetAllActorsOfClass` "/Game/Blueprints/FinishLine.FinishLine_C"))
  (set `self.NewVar_0` (`|GetArrayItem` _outactors)))

(event `self.ReceiveActorBeginOverlap`
  (params (OtherActor :type "Actor Object Reference"))
  (`GameplayStatics.PlayWorldCameraShake` "/Game/Blueprints/CameraShakes/CS_Deneme.CS_Deneme_C" (`self.K2_GetActorLocation`) 0.0 2000.0)
  (`KismetSystemLibrary.PrintString` "Hello")
  (`KismetSystemLibrary.Delay` 4.0))

(event `self.ReceiveTick`
  (params (DeltaSeconds :type "Float (single-precision)"))
  (`KismetSystemLibrary.Delay` 1.0)
  (if (== (`self.Seconds`) 59)
    (bind _result (`/Engine/EditorBlueprintResources/StandardMacros.IncrementInt` (`self.Minutes`))
      (:`  `
        (set `self.Minutes` _result)
        (set `self.Seconds` 0)))
    (else
      (bind _result_2 (`/Engine/EditorBlueprintResources/StandardMacros.IncrementInt` (`self.Seconds`))
        (:`  `
          (set `self.Seconds` _result_2))))))

(fn `UserConstructionScript`)